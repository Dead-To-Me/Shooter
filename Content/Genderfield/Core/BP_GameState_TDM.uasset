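; Team deathmatch game state that scores kills and suicides and ends the match when a team reaches the goal.
; On player death, a kill adds a death to the victim and a kill and bonus points to the killer, while a suicide only deducts penalty points.
; Each kill also increments the killer's team score during the Playing state, then checks both teams against GameGoal to call EndMatch.
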(event `self.OnPlayerDead_Event`
  (params (DeadPlayer :type "Controller Object Reference") (Killer :type "Controller Object Reference") (DamageCauser :type "Actor Object Reference"))
  (bind _playerstate (`Controller.PlayerState` Killer))
  (bind _playerstate_2 (`Controller.PlayerState` DeadPlayer))
  (bind _splayerstate (message `/Game/Genderfield/Core/Interfaces/BPI_SPlayerState.GetSPlayerState` _playerstate_2))
  (bind _splayerstate_2 (message `/Game/Genderfield/Core/Interfaces/BPI_SPlayerState.GetSPlayerState` _playerstate))
  (if (!= _playerstate_2 _playerstate)
    (`|ExecutionSequence`
      (:`then_0`
        (`/Engine/EditorBlueprintResources/StandardMacros.IncrementInt` (`SPlayerState.Deaths` _splayerstate)))
      (:`then_1`
        (set `SPlayerState.Points` (+ (`SPlayerState.Points` _splayerstate_2) (`self.BonusPointAfterKill`)) _splayerstate_2)
        (`/Engine/EditorBlueprintResources/StandardMacros.IncrementInt` (`SPlayerState.Kills` _splayerstate_2)
          (:`  `
            (`self.AddCurrentGoalTDM` (`SPlayerState.Team` _splayerstate_2))))))
    (else
      (set `SPlayerState.Points` (- (`SPlayerState.Points` _splayerstate_2) (`self.PenaltySuicide`)) _splayerstate_2))))

(event `self.AddCurrentGoal`
  (if (>= (`self.TeamAPoints`) (`self.GameGoal`))
    (`self.EndMatch`)
    (elif (>= (`self.TeamBPoints`) (`self.GameGoal`))
      (`self.EndMatch`))))

(event `AddCurrentGoalTDM`
  (params (Team :type "ETeams Enum" :default "TeamA"))
  (switch `EMatchState` (`self.MatchState`)
    (:`Playing`
      (`|ExecutionSequence`
        (:`then_0`
          (switch `ETeams` Team
            (:`TeamA`
              (`/Engine/EditorBlueprintResources/StandardMacros.IncrementInt` (`self.TeamAPoints`)))
            (:`TeamB`
              (`/Engine/EditorBlueprintResources/StandardMacros.IncrementInt` (`self.TeamBPoints`)))))
        (:`then_1`
          (`self.AddCurrentGoal`))))))

(fn `UserConstructionScript`
  (`parent.UserConstructionScript`))