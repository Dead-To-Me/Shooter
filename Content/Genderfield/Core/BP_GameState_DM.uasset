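; Deathmatch GameState that scores player deaths when the OnPlayerDeadEvent event fires.
; It reads each player's stats through GetSPlayerStateMessage on their PlayerState.
; A kill calls AddCurrentGoal, increments the victim's Deaths and the killer's Kills, and adds BonusPointAfterKill to the killer's Points.
; A suicide, detected by matching PlayerStates, only subtracts PenaltySuicide from Points, leaving Deaths and the goal untouched.
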(event `self.ReceiveBeginPlay`
  (`parent.ReceiveBeginPlay`))

(event `self.OnPlayerDead_Event`
  (params (DeadPlayer :type "Controller Object Reference") (Killer :type "Controller Object Reference") (DamageCauser :type "Actor Object Reference"))
  (bind _playerstate (`Controller.PlayerState` DeadPlayer))
  (bind _playerstate_2 (`Controller.PlayerState` Killer))
  (bind _splayerstate (message `/Game/Genderfield/Core/Interfaces/BPI_SPlayerState.GetSPlayerState` _playerstate))
  (bind _splayerstate_2 (message `/Game/Genderfield/Core/Interfaces/BPI_SPlayerState.GetSPlayerState` _playerstate_2))
  (if (!= _playerstate _playerstate_2)
    (`self.AddCurrentGoal`)
    (`|ExecutionSequence`
      (:`then_0`
        (`/Engine/EditorBlueprintResources/StandardMacros.IncrementInt` (`SPlayerState.Deaths` _splayerstate)))
      (:`then_1`
        (set `SPlayerState.Points` (+ (`SPlayerState.Points` _splayerstate_2) (`self.BonusPointAfterKill`)) _splayerstate_2)
        (`/Engine/EditorBlueprintResources/StandardMacros.IncrementInt` (`SPlayerState.Kills` _splayerstate_2))))
    (else
      (set `SPlayerState.Points` (- (`SPlayerState.Points` _splayerstate_2) (`self.PenaltySuicide`)) _splayerstate_2))))

(fn `UserConstructionScript`
  (`parent.UserConstructionScript`))