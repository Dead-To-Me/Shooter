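; BP_GameMode_TDM is a team deathmatch game mode that picks spawn points by team.
; FindPlayerStart reads the player's team from the player state and gathers BP_SPlayerStart actors whose tag matches that team's name.
; It returns the first one that reports it can be used, otherwise it prints a debug message and falls back to a random start from the team's set.
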(fn `FindPlayerStart`
  (params (Player :type "Controller Object Reference") (IncomingName :type String))
  (returns (ReturnValue :type "Actor Object Reference"))
  (bind _splayerstate (message `/Game/Genderfield/Core/Interfaces/BPI_SPlayerState.GetSPlayerState` (`Controller.PlayerState` Player)))
  (bind _outactors (`GameplayStatics.GetAllActorsOfClassWithTag` "/Game/Genderfield/Core/Base/BP_SPlayerStart.BP_SPlayerStart_C" (`KismetStringLibrary.Conv_StringToName` (`|GetEnumeratorNameAsString` (`SPlayerState.Team` _splayerstate)))))
  (for _array_element _outactors
    (if (`/Game/Genderfield/Core/Base/BP_SPlayerStart.CanBeUsed` _array_element)
      (return _array_element)))
  (`KismetSystemLibrary.PrintString` "Seelct Random Player Start ================================================" false)
  (return (`KismetArrayLibrary.Array_Random` _outactors)))

(fn `UserConstructionScript`
  (`parent.UserConstructionScript`))