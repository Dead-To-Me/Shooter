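; BP_ControlPoint is a control point for the team deathmatch game state, awarding goal score to the team that captured it.
; AddTeamScore scores only while captured with unequal team player counts; a tie switches it to Resisting and ensures a looping CapturingPoint timer runs.
; Match end, received through the game state's delegate, clears both capture timers.
; Tick prints player counts and point state for debugging.
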(event `self.ReceiveBeginPlay`
  (bind _asbp_game_state_tdm (cast `/Game/Genderfield/Core/BP_GameState_TDM` (`GameplayStatics.GetGameState`)))
  (bind _output_get (set `self.GameStateTDM` _asbp_game_state_tdm))
  (add `/Game/Genderfield/Core/Base/BP_GameState.OnMatchStateChanged` _output_get (delegate `OnMatchStateChanged_Event`)))

(event `OnMatchStateChanged_Event`
  (params (MatchState :type "EMatchState Enum" :default "Preparation"))
  (switch `EMatchState` MatchState
    (:`End`
      (`KismetSystemLibrary.K2_ClearAndInvalidateTimerHandle` (`self.CaptureTimer`))
      (`KismetSystemLibrary.K2_ClearAndInvalidateTimerHandle` (`self.CapturingTimer`)))))

(event `self.ReceiveTick`
  (params (DeltaSeconds :type "Float (single-precision)"))
  (`KismetSystemLibrary.PrintString` (`KismetStringLibrary.Concat_StrStr` (`KismetStringLibrary.Conv_IntToString` (`self.TeamAPlayers`)) "   " (`KismetStringLibrary.Conv_IntToString` (`self.TeamBPlayers`)) "  " (`|GetEnumeratorNameAsString` (`self.ControlPointState`))) true false (struct :`G` 0.66 :`B` 1.0 :`A` 1.0) 0.01))

(event `self.AddTeamScore`
  (switch `EControlPointState` (`self.ControlPointState`)
    (:`Captured`
      (if (!= (`self.TeamAPlayers`) (`self.TeamBPlayers`))
        (bind _gamestatetdm (`self.GameStateTDM`)
          (:`then`
            (`/Game/Genderfield/Core/BP_GameState_TDM.AddCurrentGoalTDM` _gamestatetdm (`self.CurrentCaptureTeam`)))
          (:`else`))
        (else
          (set `self.ControlPointState` "Resisting")
          (if (not (`KismetSystemLibrary.K2_IsValidTimerHandle` (`self.CapturingTimer`)))
            (bind _returnvalue (`KismetSystemLibrary.K2_SetTimer` null "CapturingPoint" 0.0 true))
            (set `self.CapturingTimer` _returnvalue)))))))

(event `self.ClientsOnChangedControlTeam`)

(fn `UserConstructionScript`)