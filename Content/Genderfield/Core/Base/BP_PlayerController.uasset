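; Player controller blueprint that routes pause and scoreboard input to the HUD and handles leaving the game.
; Pause input toggles the pause menu through the HUD's SHUDMessage, while holding the Scoreboard input shows the main HUD's scoreboard widget and releasing hides it.
; LeaveGame destroys the online session, and GetSPlayerController returns the controller itself.
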(event `LeaveGame`
  (`DestroySessionCallbackProxy.DestroySession` self))

(event `InputAction|PauseMenu`
  (params (Key :type "Key Structure"))
  (:`Pressed`
    (bind _getshud (message `/Game/Genderfield/Core/Interfaces/BPI_SHUD.GetSHUD` (`self.GetHUD`)))
    (`SHUD.TogglePauseMenu` _getshud)))

(event `InputAction|Scoreboard`
  (params (Key :type "Key Structure"))
  (:`Pressed`
    (bind _getshud (message `/Game/Genderfield/Core/Interfaces/BPI_SHUD.GetSHUD` (`self.GetHUD`)))
    (bind _scoreboard (`/Game/Genderfield/Widgets/WBP_MainHUD.Scoreboard` (`/Game/Genderfield/Core/Base/BP_HUD.MainHUD` _getshud))
      (:`then`
        (`Widget.SetVisibility` _scoreboard "Visible"))
      (:`else`)))
  (:`Released`
    (bind _getshud_2 (message `/Game/Genderfield/Core/Interfaces/BPI_SHUD.GetSHUD` (`self.GetHUD`)))
    (bind _scoreboard_2 (`/Game/Genderfield/Widgets/WBP_MainHUD.Scoreboard` (`/Game/Genderfield/Core/Base/BP_HUD.MainHUD` _getshud_2))
      (:`then`
        (`Widget.SetVisibility` _scoreboard_2 "Hidden"))
      (:`else`))))

(fn `GetSPlayerController`
  (returns (GetSPlayerController :type "/Game/Genderfield/Core/Base/BP_PlayerController Object Reference"))
  (return self))

(fn `UserConstructionScript`)