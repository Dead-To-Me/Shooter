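; Base player character for a team shooter, handling client-side cosmetic setup, minimap, camera FOV and recoil.
; On non-authority BeginPlay it applies the team flag patch, then wires the local player's minimap render target or other players' tag and relation-coloured icon.
; Enemy icons follow replicated detection, and a timeline turns recoil into controller input.
; Keys toggle AK-110 skins and night vision; head-following camera code is disconnected, marked for C++.
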(event `self.ReceiveTick`
  (params (DeltaSeconds :type "Float (single-precision)")))

(event `self.ReceiveBeginPlay`
  (`/Engine/EditorBlueprintResources/ActorMacros.Switch Has Authority`
    (:`Remote`
      (bind _splayerstate (message `/Game/Genderfield/Core/Interfaces/BPI_SPlayerState.GetSPlayerState` (`self.PlayerState`)))
      (set `self.Flag` (select `ETeams` (`SPlayerState.Team` _splayerstate) :`TeamA` "/Game/Genderfield/Cassandra/Textures/T_RF.T_RF" :`TeamB` "/Game/Genderfield/Cassandra/Textures/T_USA_Flag.T_USA_Flag" :!type "Texture Object Reference"))
      (if (`self.IsLocallyControlled`)
        (bind _returnvalue (`PrimitiveComponent.CreateDynamicMaterialInstance` (`self.OwnerMesh`) 4 "/Game/Genderfield/Cassandra/Materials/MI_Cassandra_Patch.MI_Cassandra_Patch" "None"))
        (`MaterialInstanceDynamic.SetTextureParameterValue` _returnvalue "Flag" (`self.Flag`))
        (bind _getgameinstacne (message `/Game/Genderfield/Core/Interfaces/BPI_GameInstacne.GetGameInstace` (`GameplayStatics.GetGameInstance`)))
        (set `self.FieldOfViewScope` (`/Game/Genderfield/Core/Base/BP_SaveGame.FOVScope` (`/Game/Genderfield/Core/Base/BP_GameInstace.SaveGame` _getgameinstacne)))
        (bind _getsplayercontroller (message `/Game/Genderfield/Core/Interfaces/BPI_SPlayerContreoller.GetSPlayerController` (`self.GetController`)))
        (`WidgetBlueprintLibrary.SetInputMode_GameOnly` _getsplayercontroller)
        (set `PlayerController.bShowMouseCursor` false _getsplayercontroller)
        (bind _returnvalue_2 (`KismetRenderingLibrary.CreateRenderTarget2D` 256))
        (bind _output_get (set `SceneCaptureComponent2D.TextureTarget` _returnvalue_2 (`self.MapCapture`)))
        (bind _getshud (message `/Game/Genderfield/Core/Interfaces/BPI_SHUD.GetSHUD` (`PlayerController.GetHUD` _getsplayercontroller)))
        (bind _returnvalue_3 (`Border.GetDynamicMaterial` (`/Game/Genderfield/Widgets/WBP_Minimap.MinimapBorder` (`/Game/Genderfield/Widgets/WBP_MainHUD.WBP_Minimap` (`/Game/Genderfield/Core/Base/BP_HUD.MainHUD` _getshud)))))
        (`MaterialInstanceDynamic.SetTextureParameterValue` _returnvalue_3 "MapTexture" _output_get)
        (else
          (bind _returnvalue_4 (`PrimitiveComponent.CreateDynamicMaterialInstance` (`self.Mesh`) 4 "/Game/Genderfield/Cassandra/Materials/MI_Cassandra_Patch.MI_Cassandra_Patch" "None"))
          (`MaterialInstanceDynamic.SetTextureParameterValue` _returnvalue_4 "Flag" (`self.Flag`))
          (bind _aswbp_player_tag (cast `/Game/Genderfield/Widgets/WBP_PlayerTag` (`WidgetComponent.GetUserWidgetObject` (`self.PlayerBarWidget`))))
          (set `SPlayerTagWidget.Player` self _aswbp_player_tag)
          (bind _splayerstate_2 (message `/Game/Genderfield/Core/Interfaces/BPI_SPlayerState.GetSPlayerState` (`self.PlayerState`)))
          (bind _splayerstate_3 (message `/Game/Genderfield/Core/Interfaces/BPI_SPlayerState.GetSPlayerState` (`GameplayStatics.GetPlayerState` 0)))
          (bind _returnvalue_5 (`SPlayerState.GetRelation` _splayerstate_3 _splayerstate_2))
          (`PaperSpriteComponent.SetSpriteColor` (`self.PlayerIcon`) (select `ERelation` _returnvalue_5 :`Enemy` (struct :`R` 1.0 :`G` 0.1 :`B` 0.1 :`A` 1.0) :`Ally` (struct :`R` 0.1 :`G` 0.1 :`B` 1.0 :`A` 1.0) :`Friend` (struct :`R` 0.1 :`G` 1.0 :`B` 0.1 :`A` 1.0) :!type "LinearColor Structure"))
          (`PaperSpriteComponent.SetSprite` (`self.PlayerIcon`) (select `ERelation` _returnvalue_5 :`Ally` "/Game/Genderfield/Textures/S_PlayerIcon.S_PlayerIcon" :`Friend` "/Game/Genderfield/Textures/S_PlayerIcon.S_PlayerIcon" :!type "PaperSprite Object Reference")))))))

(event `/Game/Genderfield/Core/Interfaces/BPI_GameInstacne.SetFieldOfView`
  (params (FOV :type "Float (double-precision)"))
  (bind _output_get (set `self.FieldOfView` FOV))
  (`CameraComponent.SetFieldOfView` (`self.Camera`) _output_get)
  (bind _getsplayercontroller (message `/Game/Genderfield/Core/Interfaces/BPI_SPlayerContreoller.GetSPlayerController` (`self.GetController`)))
  (`SPlayerController.OnFOVChanged` _getsplayercontroller (`self.FieldOfView`)))

(event `/Game/Genderfield/Core/Interfaces/BPI_GameInstacne.SetFieldOfViewScope`
  (params (FOV :type "Float (double-precision)"))
  (set `self.FieldOfViewScope` FOV))

(event `InputAction|ChangeSkin`
  (params (Key :type "Key Structure"))
  (:`Pressed`
    (bind _asbp_weapon_ak_110 (cast `/Game/Genderfield/Weapons/AK-110/BP_Weapon_AK-110` (`SWeaponManagerComponent.GetCurrentWeapon` (`self.WeaponManager`))))
    (`/Engine/EditorBlueprintResources/StandardMacros.FlipFlop`
      (:`A`
        (bind _weaponmesh (`SWeapon.WeaponMesh` _asbp_weapon_ak_110))
        (`PrimitiveComponent.SetMaterial` _weaponmesh 0 "/Game/Genderfield/Weapons/AK-110/Material/MI_AK-110_Skin_Ser.MI_AK-110_Skin_Ser"))
      (:`B`
        (`PrimitiveComponent.SetMaterial` _weaponmesh 0 "/Game/Genderfield/Weapons/AK-110/Material/M_AK-110_MysticRain_Mat_Inst.M_AK-110_MysticRain_Mat_Inst")))))

(event `self.AddRecoil`
  (params (Recoil :type "Vector2D Structure (by ref)"))
  (bind (_direction _alpha) (`Timeline|Timeline` :!via `PlayFromStart`)
    (:`Update`
      (`self.AddControllerPitchInput` (`KismetMathLibrary.Lerp` 0.0 Recoil_X _alpha))
      (`self.AddControllerYawInput` (`KismetMathLibrary.Lerp` 0.0 Recoil_Y _alpha)))))

(event `self.OnRepDetected`
  (if (not (`self.IsLocallyControlled`))
    (bind _splayerstate (message `/Game/Genderfield/Core/Interfaces/BPI_SPlayerState.GetSPlayerState` (`self.PlayerState`)))
    (bind _splayerstate_2 (message `/Game/Genderfield/Core/Interfaces/BPI_SPlayerState.GetSPlayerState` (`GameplayStatics.GetPlayerState` 0)))
    (switch `ERelation` (`SPlayerState.GetRelation` _splayerstate_2 _splayerstate)
      (:`Enemy`
        (`PaperSpriteComponent.SetSprite` (`self.PlayerIcon`) (select `bool` (`self.bDetected`) :`true` "/Game/Genderfield/Textures/S_PlayerIcon.S_PlayerIcon" :!type "PaperSprite Object Reference"))))))

(event `Key|T`
  (params (Key :type "Key Structure"))
  (:`Pressed`
    (`/Engine/EditorBlueprintResources/StandardMacros.FlipFlop`
      (:`A`
        (set `CameraComponent.PostProcessSettings` (`self.NightVisionPP`) (`self.Camera`)))
      (:`B`
        (set `CameraComponent.PostProcessSettings` (`self.DefaultPP`) (`self.Camera`))))))

(fn `GetGameInstace`
  (returns (GetGameInstacne :type "/Game/Genderfield/Core/Base/BP_GameInstace Object Reference"))
  (return null))

(fn `GetSCharacter`
  (returns (BP_SCharacter :type "/Game/Genderfield/Core/Base/BP_SCharacter Object Reference"))
  (return self))

(fn `UserConstructionScript`)