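; Player camera manager that shows a directional on-hit post-process effect when the owning player takes damage.
; On non-server instances, BeginPlay binds to the player controller message's damage event and creates a dynamic MI_OnHit material.
; Each hit adds that material as a blendable on the pawn's camera and converts the damage direction into offset control-rotation space for its Direction parameter.
; A restarted timeline animates the material's Alpha.
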(event `self.ReceiveBeginPlay`
  (if (not (`KismetSystemLibrary.IsServer`))
    (bind _getsplayercontroller (message `/Game/Genderfield/Core/Interfaces/BPI_SPlayerContreoller.GetSPlayerController` (`self.GetOwningPlayerController`)))
    (add `SPlayerController.OnPlayerDamage` _getsplayercontroller (delegate `OnPlayerDamage_Event`))
    (bind _returnvalue (`KismetMaterialLibrary.CreateDynamicMaterialInstance` "/Game/Genderfield/Materials/MI_OnHit.MI_OnHit"))
    (set `self.M_OnDamage` _returnvalue)))

(event `OnPlayerDamage_Event`
  (params (Direction :type "Vector Structure"))
  (bind _bp_scharacter (message `/Game/Genderfield/Core/Interfaces/BPI_SCharacter.GetSCharacter` (`Controller.K2_GetPawn` (`self.GetOwningPlayerController`))))
  (`CameraComponent.AddOrUpdateBlendable` (`SCharacter.Camera` _bp_scharacter) (`self.M_OnDamage`) 1.0)
  (`MaterialInstanceDynamic.SetVectorParameterValue` (`self.M_OnDamage`) "Direction" (`KismetMathLibrary.Conv_VectorToLinearColor` (`KismetMathLibrary.LessLess_VectorRotator` Direction (`KismetMathLibrary.ComposeRotators` (`Controller.GetControlRotation` (`self.GetOwningPlayerController`)) (struct :`Yaw` 90.0)))))
  (bind (_direction _apha) (`Timeline|OnDamageAlphaTimeline` :!via `PlayFromStart`)
    (:`Update`
      (`MaterialInstanceDynamic.SetScalarParameterValue` (`self.M_OnDamage`) "Alpha" _apha))))

(fn `UserConstructionScript`)