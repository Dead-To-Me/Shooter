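; BP_GameState is the game state Blueprint that relays match state and map vote changes through event calls.
; On the authority, BeginPlay binds to the game mode's player-death message, though that handler is currently empty.
; Match state replication calls OnMatchStateChanged, and the map vote multicast calls OnMapVoteCountChanged on remote machines only.
; GetSGameState returns the state itself.
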(event `self.ReceiveBeginPlay`
  (`/Engine/EditorBlueprintResources/ActorMacros.Switch Has Authority`
    (:`Authority`
      (bind _gamemode (message `/Game/Genderfield/Core/Interfaces/BPI_GameMode.GetGameMode` (`GameplayStatics.GetGameMode`)))
      (add `SGameModeBase.OnPlayerDead` _gamemode (delegate `OnPlayerDead_Event`)))))

(event `OnPlayerDead_Event`
  (params (DeadPlayer :type "Controller Object Reference") (Killer :type "Controller Object Reference") (DamageCauser :type "Actor Object Reference")))

(event `self.OnRep_MatchState`
  (`self.OnMatchStateChanged` (`self.MatchState`)))

(event `self.MulticastMapVoteCountUpdateBlueprint`
  (params (MapIndex :type Integer) (VoteCount :type Integer))
  (`/Engine/EditorBlueprintResources/ActorMacros.Switch Has Authority`
    (:`Remote`
      (`self.OnMapVoteCountChanged` MapIndex VoteCount))))

(fn `GetSGameState`
  (returns (SGameState :type "/Game/Genderfield/Core/Base/BP_GameState Object Reference"))
  (return self))

(fn `UserConstructionScript`)