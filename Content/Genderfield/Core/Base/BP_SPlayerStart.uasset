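; Team-based player start that refuses spawns while an opposing team's character is nearby.
; Construction writes the Team enum name into the first actor tag.
; CanBeUsed checks characters overlapping the Box, comparing their PlayerState team through message getters, and locks the start if any differs.
; A retriggerable delay clears the lock shortly afterwards; calls made while locked return false without rechecking.
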(event `SetLockedRetriggerableDelay`
  (`KismetSystemLibrary.RetriggerableDelay` 1.5)
  (set `self.bLocked` false))

(fn `CanBeUsed`
  (returns (CanUse :type Boolean))
  (if (not (`self.bLocked`))
    (for _array_element (`PrimitiveComponent.GetOverlappingActors` (`self.Box`) "/Game/Genderfield/Core/Base/BP_SCharacter.BP_SCharacter_C")
      (bind _bp_scharacter (message `/Game/Genderfield/Core/Interfaces/BPI_SCharacter.GetSCharacter` _array_element))
      (bind _splayerstate (message `/Game/Genderfield/Core/Interfaces/BPI_SPlayerState.GetSPlayerState` (`Pawn.PlayerState` _bp_scharacter)))
      (if (`|EnumInequality` (`SPlayerState.Team` _splayerstate) (`self.Team`))
        (set `self.bLocked` true)
        (break)))
    (`self.SetLockedRetriggerableDelay`)
    (return (not (`self.bLocked`)))
    (else
      (return false))))

(fn `UserConstructionScript`
  (bind _tags (`self.Tags`))
  (if (`KismetArrayLibrary.Array_IsValidIndex` _tags)
    (`KismetArrayLibrary.Array_Set` _tags 0 (`KismetStringLibrary.Conv_StringToName` (`|GetEnumeratorNameAsString` (`self.Team`))))
    (else
      (`KismetArrayLibrary.Array_Add` _tags (`KismetStringLibrary.Conv_StringToName` (`|GetEnumeratorNameAsString` (`self.Team`)))))))