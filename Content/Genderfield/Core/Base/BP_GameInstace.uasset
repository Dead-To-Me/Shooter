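; Game instance that owns the player's settings save object, loading or creating it on Init and writing it to its slot on Shutdown.
; Setters store FOV, sensitivity, mouse inversion, kill feed and FPS options in that object, with mouse and aim changes also pushed to SPlayerController.
; The FPS display setter runs the "stat fps" toggle command regardless of the requested state.
; SetSoundMix only prints, and SetArsenalSlots is an empty stub.
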(event `self.ReceiveInit`
  (bind _returnvalue (`GameplayStatics.DoesSaveGameExist` (`self.SaveGameSlot`)))
  (if _returnvalue
    (bind _returnvalue_2 (`GameplayStatics.LoadGameFromSlot` (`self.SaveGameSlot`)))
    (bind _asbp_save_game (cast `/Game/Genderfield/Core/Base/BP_SaveGame` _returnvalue_2))
    (set `self.SaveGame` _asbp_save_game)
    (else
      (bind _returnvalue_3 (`GameplayStatics.CreateSaveGameObject` "/Game/Genderfield/Core/Base/BP_SaveGame.BP_SaveGame_C"))
      (set `self.SaveGame` _returnvalue_3))))

(event `self.ReceiveShutdown`
  (`GameplayStatics.SaveGameToSlot` (`self.SaveGame`) (`self.SaveGameSlot`)))

(event `SetSoundMix`
  (`KismetSystemLibrary.PrintString` "SetSoundMix"))

(event `/Game/Genderfield/Core/Interfaces/BPI_GameInstacne.SetFieldOfViewScope`
  (params (FOV :type "Float (double-precision)"))
  (bind _savegame (`self.SaveGame`)
    (:`then`
      (set `/Game/Genderfield/Core/Base/BP_SaveGame.FOVScope` FOV _savegame))
    (:`else`)))

(event `/Game/Genderfield/Core/Interfaces/BPI_GameInstacne.SetFieldOfView`
  (params (FOV :type "Float (double-precision)"))
  (bind _savegame (`self.SaveGame`)
    (:`then`
      (set `/Game/Genderfield/Core/Base/BP_SaveGame.FOV` FOV _savegame))
    (:`else`)))

(fn `GetGameInstace`
  (returns (GetGameInstacne :type "/Game/Genderfield/Core/Base/BP_GameInstace Object Reference"))
  (return self))

(fn `SetAimSens`
  (params (AimSens :type "Float (double-precision)") (PC :type "PlayerController Object Reference"))
  (bind _savegame (`self.SaveGame`)
    (:`then`
      (bind _output_get (set `/Game/Genderfield/Core/Base/BP_SaveGame.AimSens` AimSens _savegame))
      (bind _assplayer_controller (cast `SPlayerController` PC)
        (:`then`
          (`SPlayerController.SetAimSens` _assplayer_controller _output_get)
          (return))
        (:`CastFailed`
          _)))
    (:`else`
      _))
  (`KismetSystemLibrary.PrintString` "SetAimSens: SaveGame Invalid"))

(fn `SetArsenalSlots`
  (params (ArsenalSlots :type "InventorySlots Structure (by ref)"))
  (return))

(fn `SetFPS`
  (params (FPS :type "Float (double-precision)"))
  (bind _savegame (`self.SaveGame`)
    (:`then`
      (set `/Game/Genderfield/Core/Base/BP_SaveGame.FPS` FPS _savegame))
    (:`else`)))

(fn `SetMouseInverted`
  (params (bInverted :type Boolean) (PC :type "PlayerController Object Reference"))
  (bind _savegame (`self.SaveGame`)
    (:`then`
      (bind _output_get (set `/Game/Genderfield/Core/Base/BP_SaveGame.bMouseInverted` bInverted _savegame))
      (bind _assplayer_controller (cast `SPlayerController` PC))
      (`SPlayerController.SetMouseInverted` _assplayer_controller _output_get))
    (:`else`)))

(fn `SetMouseSens`
  (params (Sens :type "Float (double-precision)") (PC :type "PlayerController Object Reference"))
  (bind _assplayer_controller (cast `SPlayerController` PC))
  (bind _savegame (`self.SaveGame`)
    (:`then`
      (bind _output_get (set `/Game/Genderfield/Core/Base/BP_SaveGame.MouseSens` Sens _savegame))
      (`SPlayerController.SetMouseSensitivity` _assplayer_controller _output_get))
    (:`else`)))

(fn `SetShowFPS`
  (params (bEnabled :type Boolean))
  (bind _savegame (`self.SaveGame`)
    (:`then`
      (set `/Game/Genderfield/Core/Base/BP_SaveGame.bShowFPS` bEnabled _savegame)
      (`KismetSystemLibrary.ExecuteConsoleCommand` "stat fps" (`GameplayStatics.GetPlayerController` 0)))
    (:`else`)))

(fn `SetShowKillFeed`
  (params (bShowKillFeed :type Boolean))
  (bind _savegame (`self.SaveGame`)
    (:`then`
      (set `/Game/Genderfield/Core/Base/BP_SaveGame.bKillFeed` bShowKillFeed _savegame))
    (:`else`)))