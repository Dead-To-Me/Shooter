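; Exploding grenade actor that provides the detonation entry point and local widget feedback.
; ExplodeGrenade calls MulticastExplodeGrenade only while the Exploded flag is unset; the multicast event is empty here and the flag is not set in this graph.
; ShowInteractWidget plays the WBP_Grenade animation on the grenade's widget, only when the instigator's controller is local.
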(event `self.ExplodeGrenade`
  (if (not (`self.bExploded`))
    (`self.MulticastExplodeGrenade`)))

(event `MulticastExplodeGrenade`)

(event `SInteractInterface.ShowInteractWidget`
  (bind _returnvalue (`self.GetInstigatorController`))
  (`/Engine/EditorBlueprintResources/StandardMacros.IsValid` _returnvalue
    (:`Is Valid`
      (if (`Controller.IsLocalController` _returnvalue)
        (bind _aswbp_grenade (cast `/Game/Genderfield/Widgets/WBP_Grenade` (`WidgetComponent.GetUserWidgetObject` (`self.GrenadeWidget`))))
        (`/Game/Genderfield/Widgets/WBP_Grenade.PlayGrenadeAnim` _aswbp_grenade)))))

(fn `UserConstructionScript`)