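; BP_Grenade_Incendiary is an incendiary grenade that leaves a damage area for ten seconds after exploding.
; ExplodeGrenade calls a multicast event that splits by authority.
; Authority enables overlaps on Cylinder, zeroes its relative rotation and loops a timer applying point damage to overlapping actors, cleared on destruction.
; Remotes only hide the mesh and spawn the explosion effect, so a listen-server host gets neither.
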(event `self.ExplodeGrenade`
  (`self.MuticastExplodeGrenade`))

(event `MuticastExplodeGrenade`
  (`self.SetLifeSpan` 10.0)
  (`/Engine/EditorBlueprintResources/ActorMacros.Switch Has Authority`
    (:`Authority`
      (set `PrimitiveComponent.bGenerateOverlapEvents` true (`self.Cylinder`))
      (bind _returnvalue (`KismetSystemLibrary.K2_SetTimerDelegate` (delegate `Damage`) 0.25 true))
      (set `self.DamageTimer` _returnvalue)
      (`SceneComponent.K2_SetRelativeRotation` :`self` (`self.Cylinder`)))
    (:`Remote`
      (`SceneComponent.SetVisibility` (`self.GrenadeMesh`) false false)
      (`NiagaraFunctionLibrary.SpawnSystemAtLocation` (`self.ExplosionSystem`) (`self.K2_GetActorLocation`)))))

(event `Damage`
  (for _array_element (`PrimitiveComponent.GetOverlappingActors` (`self.Cylinder`) "/Script/Engine.Actor")
    (`GameplayStatics.ApplyPointDamage` _array_element 7.5 (`KismetMathLibrary.MakeVector` 0.0) (`GameplayStatics.MakeHitResult` false) (`self.GetInstigatorController`) self)))

(event `self.ReceiveDestroyed`
  (`KismetSystemLibrary.K2_ClearAndInvalidateTimerHandle` (`self.DamageTimer`)))

(fn `UserConstructionScript`)