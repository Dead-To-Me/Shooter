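; Smoke grenade actor that replaces its mesh with a Niagara smoke cloud when it explodes.
; ExplodeGrenade calls MuticastExplodeGrenade, which hides the mesh, sets a fixed lifespan and spawns the cloud at the grenade's location.
; The cloud spawns only on the Remote (non-authority) branch, so the authority never creates it.
; When the actor is destroyed, that same branch destroys the stored smoke component, tying the cloud to the grenade's lifespan.
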(event `self.ExplodeGrenade`
  (`self.MuticastExplodeGrenade`))

(event `MuticastExplodeGrenade`
  (`self.SetLifeSpan` 15.0)
  (`SceneComponent.SetVisibility` (`self.GrenadeMesh`) false false)
  (`/Engine/EditorBlueprintResources/ActorMacros.Switch Has Authority`
    (:`Remote`
      (bind _returnvalue (`NiagaraFunctionLibrary.SpawnSystemAtLocation` "/Game/Genderfield/Particles/NS_SmokeCloud1.NS_SmokeCloud1" (`self.K2_GetActorLocation`)))
      (set `self.NS_Smoke` _returnvalue))))

(event `self.ReceiveDestroyed`
  (`/Engine/EditorBlueprintResources/ActorMacros.Switch Has Authority`
    (:`Remote`
      (`ActorComponent.K2_DestroyComponent` (`self.NS_Smoke`)))))

(fn `UserConstructionScript`)