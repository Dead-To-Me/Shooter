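; Impact grenade projectile that explodes on its first bounce or stop, whichever comes first.
; A DoOnce halts movement, hides the mesh and sets a one-second lifespan, then splits on authority.
; The authority applies radial falloff damage from slightly above the grenade, crediting the instigator.
; Only remote instances play the Niagara explosion, sound and camera shake, so an authority instance, including a listen-server host's, spawns no effects here.
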(event `self.ProjectileMovement.OnProjectileBounce`
  (params (ImpactResult :type "HitResult Structure (by ref)") (ImpactVelocity :type "Vector Structure (by ref)"))
  (bind (_returnvalue_x _returnvalue_y _returnvalue_z) (`KismetMathLibrary.BreakVector` (`self.K2_GetActorLocation`)))
  (bind _returnvalue (`self.K2_GetActorLocation`))
  (`/Engine/EditorBlueprintResources/StandardMacros.DoOnce` false :!label _label
    (:`Completed`
      (set `MovementComponent.Velocity` (0.0 0.0 0.0) (`self.ProjectileMovement`))
      (`self.SetLifeSpan` 1.0)
      (`SceneComponent.SetVisibility` (`self.GrenadeMesh`) false false)
      (`/Engine/EditorBlueprintResources/ActorMacros.Switch Has Authority`
        (:`Authority`
          (`GameplayStatics.ApplyRadialDamageWithFalloff` :`BaseDamage` (`self.MaxDamage`) :`MinimumDamage` (`self.MinDamage`) :`Origin` (`KismetMathLibrary.MakeVector` _returnvalue_x _returnvalue_y (+ _returnvalue_z 15.0)) :`DamageInnerRadius` (`self.DamageInnerRadius`) :`DamageOuterRadius` (`self.DamageOuterRadius`) :`DamageFalloff` (`self.DamageFalloff`) :`DamageCauser` self :`InstigatedByController` (`self.GetInstigatorController`)))
        (:`Remote`
          (`NiagaraFunctionLibrary.SpawnSystemAtLocation` "/Game/Genderfield/Particles/NS_Explosion_Frag_small.NS_Explosion_Frag_small" (`self.K2_GetActorLocation`))
          (`GameplayStatics.SpawnSoundAtLocation` "/Game/Genderfield/Sounds/Explosion/A_Explosion_Grenade.A_Explosion_Grenade" _returnvalue (struct) 1.0 1.0 0.0 null null)
          (`GameplayStatics.PlayWorldCameraShake` "/Game/Genderfield/Data/CS_Explosion.CS_Explosion_C" _returnvalue (* (`self.DamageInnerRadius`) 2.0) (* (`self.DamageOuterRadius`) 1.5) (`self.DamageFalloff`)))))))

(event `self.ProjectileMovement.OnProjectileStop`
  (params (ImpactResult :type "HitResult Structure (by ref)"))
  (goto _label))

(fn `UserConstructionScript`)