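; Frag grenade Blueprint that implements the explosion through the MulticastExplodeGrenade event.
; On detonation it hides the grenade mesh, sets a short lifespan and branches on network authority.
; The authority applies radial falloff damage from slightly above the grenade, crediting the instigator controller.
; Only non-authority instances play the particle, sound and camera shake, with shake radii scaled from the damage radii.
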(event `self.MulticastExplodeGrenade`
  (bind (_returnvalue_x _returnvalue_y _returnvalue_z) (`KismetMathLibrary.BreakVector` (`self.K2_GetActorLocation`)))
  (bind _returnvalue (`self.K2_GetActorLocation`))
  (`self.SetLifeSpan` 1.0)
  (`SceneComponent.SetVisibility` (`self.GrenadeMesh`) false false)
  (`/Engine/EditorBlueprintResources/ActorMacros.Switch Has Authority`
    (:`Authority`
      (`GameplayStatics.ApplyRadialDamageWithFalloff` :`BaseDamage` (`self.MaxDamage`) :`MinimumDamage` (`self.MinDamage`) :`Origin` (`KismetMathLibrary.MakeVector` _returnvalue_x _returnvalue_y (+ _returnvalue_z 15.0)) :`DamageInnerRadius` (`self.DamageInnerRadius`) :`DamageOuterRadius` (`self.DamageOuterRadius`) :`DamageFalloff` (`self.DamageFalloff`) :`DamageCauser` self :`InstigatedByController` (`self.GetInstigatorController`)))
    (:`Remote`
      (`NiagaraFunctionLibrary.SpawnSystemAtLocation` (`self.ExplosionSystem`) (`self.K2_GetActorLocation`))
      (`GameplayStatics.SpawnSoundAtLocation` (`self.ExplosionSound`) _returnvalue (struct) 1.0 1.0 0.0 null null)
      (`GameplayStatics.PlayWorldCameraShake` "/Game/Genderfield/Data/CS_Explosion.CS_Explosion_C" _returnvalue (* (`self.DamageInnerRadius`) 2.0) (* (`self.DamageOuterRadius`) 1.5) (`self.DamageFalloff`)))))

(fn `UserConstructionScript`
  (`parent.UserConstructionScript`))