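; Land mine world gadget that explodes when an enemy player enters its Box trigger.
; On overlap with a Player-tagged actor, it compares the instigator's and victim's player states and continues only for an Enemy relation.
; The authority applies radial damage with falloff, while remote instances spawn the explosion effect, sound and camera shake.
; Both paths then set a short life span to remove the mine.
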(event `self.Box.OnComponentBeginOverlap`
  (params (OverlappedComponent :type "PrimitiveComponent Object Reference") (OtherActor :type "Actor Object Reference") (OtherComp :type "PrimitiveComponent Object Reference") (OtherBodyIndex :type Integer) (bFromSweep :type Boolean) (SweepResult :type "HitResult Structure (by ref)"))
  (bind _returnvalue (`self.K2_GetActorLocation`))
  (if (`self.ActorHasTag` OtherActor "Player")
    (bind _bp_scharacter (message `/Game/Genderfield/Core/Interfaces/BPI_SCharacter.GetSCharacter` OtherActor))
    (bind _splayerstate (message `/Game/Genderfield/Core/Interfaces/BPI_SPlayerState.GetSPlayerState` (`Pawn.PlayerState` (`self.GetInstigator`))))
    (bind _splayerstate_2 (message `/Game/Genderfield/Core/Interfaces/BPI_SPlayerState.GetSPlayerState` (`Pawn.PlayerState` _bp_scharacter)))
    (if (`|EnumEquality` (`SPlayerState.GetRelation` _splayerstate _splayerstate_2) "Enemy")
      (`/Engine/EditorBlueprintResources/ActorMacros.Switch Has Authority`
        (:`Authority`
          (`GameplayStatics.ApplyRadialDamageWithFalloff` :`BaseDamage` (`self.MaxDamage`) :`MinimumDamage` (`self.MinDamage`) :`Origin` (`SceneComponent.K2_GetComponentLocation` (`self.Box`)) :`DamageInnerRadius` (`self.DamageInnerRadius`) :`DamageOuterRadius` (`self.DamageOuterRadius`) :`DamageFalloff` (`self.DamageFalloff`) :`DamageCauser` self :`InstigatedByController` (`self.GetInstigatorController`))
          (`self.SetLifeSpan` 0.2))
        (:`Remote`
          (`NiagaraFunctionLibrary.SpawnSystemAtLocation` (`self.ExplosionSystem`) (`self.K2_GetActorLocation`))
          (`GameplayStatics.SpawnSoundAtLocation` (`self.ExplosionSound`) _returnvalue (struct) 1.0 1.0 0.0 null null)
          (`GameplayStatics.PlayWorldCameraShake` "/Game/Genderfield/Data/CS_Explosion.CS_Explosion_C" _returnvalue (* (`self.DamageInnerRadius`) 2.0) (* (`self.DamageOuterRadius`) 1.5) (`self.DamageFalloff`))
          (`self.SetLifeSpan` 0.2))))))

(fn `UserConstructionScript`
  (`parent.UserConstructionScript`))