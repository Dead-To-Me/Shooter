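; Ammo box world gadget that resupplies a character who interacts with it.
; Interact is ignored while the cooldown timer handle is valid; otherwise it starts the cooldown.
; On the authority only, it then maxes out the character's grenades through the weapon manager and adds ammo to each weapon that manager returns.
; The CooldownEnd event is left empty.
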(event `SInteractInterface.Interact`
  (params (Character :type "SCharacter Object Reference"))
  (bind _returnvalue (`SCharacter.GetWeaponManager` Character))
  (if (not (`KismetSystemLibrary.K2_IsValidTimerHandle` (`self.CooldownTimer`)))
    (`self.BeginCooldown`)
    (`/Engine/EditorBlueprintResources/ActorMacros.Switch Has Authority`
      (:`Authority`
        (`SWeaponManagerComponent.SetMaxGrenade` _returnvalue)
        (`KismetArrayLibrary.Array_Clear` (`self.Weapons`))
        (`SWeaponManagerComponent.GetWeapons` _returnvalue (`self.Weapons`))
        (for _array_element (`self.Weapons`)
          (`SWeapon.AddAmmo` _array_element))))))

(event `self.CooldownEnd`)

(fn `UserConstructionScript`
  (`parent.UserConstructionScript`))