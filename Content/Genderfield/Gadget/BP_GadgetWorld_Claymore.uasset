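; Claymore gadget placed in the world that detonates when an enemy of its instigator crosses its trip lines.
; On authority, a looping timer line-traces along Arrow, then Arrow1 if the first misses, and compares hit player and instigator player states for an Enemy relation.
; Explode stops the timer and applies falloff radial damage on authority, spawns VFX, sound and camera shake on remotes, and sets a short lifespan.
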(event `self.ReceiveBeginPlay`
  (`parent.ReceiveBeginPlay`)
  (`/Engine/EditorBlueprintResources/ActorMacros.Switch Has Authority`
    (:`Authority`
      (bind _returnvalue (`KismetSystemLibrary.K2_SetTimerDelegate` (delegate `Check`) 0.15 true))
      (set `self.CheckTimer` _returnvalue))))

(event `Check`
  (bind _returnvalue (`SceneComponent.K2_GetComponentLocation` (`self.Arrow`)))
  (bind _returnvalue_2 (`SceneComponent.K2_GetComponentLocation` (`self.Arrow1`)))
  (bind (_outhit _returnvalue_3) (`KismetSystemLibrary.LineTraceSingle` _returnvalue (+ _returnvalue (* (`SceneComponent.GetForwardVector` (`self.Arrow`)) (`self.CheckLenght`))) "TraceTypeQuery1"))
  (if _returnvalue_3
    (bind _bp_scharacter (message `/Game/Genderfield/Core/Interfaces/BPI_SCharacter.GetSCharacter` (`.HitActor` (`GameplayStatics.BreakHitResult` _outhit))))
    (bind _splayerstate (message `/Game/Genderfield/Core/Interfaces/BPI_SPlayerState.GetSPlayerState` (`Pawn.PlayerState` _bp_scharacter)))
    (bind _splayerstate_2 (message `/Game/Genderfield/Core/Interfaces/BPI_SPlayerState.GetSPlayerState` (`Controller.PlayerState` (`self.GetInstigatorController`))))
    (if (`|EnumEquality` (`SPlayerState.GetRelation` _splayerstate _splayerstate_2) "Enemy")
      (`self.Explode`))
    (else
      (bind (_outhit_2 _returnvalue_4) (`KismetSystemLibrary.LineTraceSingle` _returnvalue_2 (+ _returnvalue_2 (* (`SceneComponent.GetForwardVector` (`self.Arrow1`)) (`self.CheckLenght`))) "TraceTypeQuery1"))
      (if _returnvalue_4
        (bind _bp_scharacter_2 (message `/Game/Genderfield/Core/Interfaces/BPI_SCharacter.GetSCharacter` (`.HitActor` (`GameplayStatics.BreakHitResult` _outhit_2))))
        (bind _splayerstate_3 (message `/Game/Genderfield/Core/Interfaces/BPI_SPlayerState.GetSPlayerState` (`Pawn.PlayerState` _bp_scharacter_2)))
        (bind _splayerstate_4 (message `/Game/Genderfield/Core/Interfaces/BPI_SPlayerState.GetSPlayerState` (`Controller.PlayerState` (`self.GetInstigatorController`))))
        (if (`|EnumEquality` (`SPlayerState.GetRelation` _splayerstate_3 _splayerstate_4) "Enemy")
          (`self.Explode`))))))

(event `Explode`
  (bind _returnvalue (`self.K2_GetActorLocation`))
  (bind _arrow1 (`self.Arrow1`))
  (`/Engine/EditorBlueprintResources/ActorMacros.Switch Has Authority`
    (:`Authority`
      (`KismetSystemLibrary.K2_ClearAndInvalidateTimerHandle` (`self.CheckTimer`))
      (`GameplayStatics.ApplyRadialDamageWithFalloff` :`BaseDamage` (`self.MaxDamage`) :`MinimumDamage` (`self.MinDamage`) :`Origin` (+ (`SceneComponent.K2_GetComponentLocation` _arrow1) (* (`SceneComponent.GetForwardVector` _arrow1) 50)) :`DamageInnerRadius` (`self.DamageInnerRadius`) :`DamageOuterRadius` (`self.DamageOuterRadius`) :`DamageFalloff` (`self.DamageFalloff`) :`DamageCauser` self :`InstigatedByController` (`self.GetInstigatorController`))
      (`self.SetLifeSpan` 0.2))
    (:`Remote`
      (`NiagaraFunctionLibrary.SpawnSystemAtLocation` (`self.ExplosionSystem`) (`self.K2_GetActorLocation`))
      (`GameplayStatics.SpawnSoundAtLocation` (`self.ExplosionSound`) _returnvalue (struct) 1.0 1.0 0.0 null null)
      (`GameplayStatics.PlayWorldCameraShake` "/Game/Genderfield/Data/CS_Explosion.CS_Explosion_C" _returnvalue (* (`self.DamageInnerRadius`) 2.0) (* (`self.DamageOuterRadius`) 1.5) (`self.DamageFalloff`))
      (`self.SetLifeSpan` 0.2))))

(fn `UserConstructionScript`
  (`parent.UserConstructionScript`))