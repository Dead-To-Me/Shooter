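; Base actor for world gadgets, providing relation-based markers, an interaction widget and stubbed Interact and cooldown-end events.
; On remote (non-authority) instances, BeginPlay compares the non-local instigator's player state with player 0's, clearing sprite and widget for enemies and tinting the sprite for allies or friends.
; It then passes texture and owner to any remaining WBP_Gadget, which ShowInteractWidget notifies.
; BeginCooldown starts a one-shot timer to CooldownEnd.
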(event `self.ReceiveBeginPlay`
  (bind _returnvalue (`self.GetInstigator`))
  (`/Engine/EditorBlueprintResources/ActorMacros.Switch Has Authority`
    (:`Remote`
      (`|ExecutionSequence`
        (:`then_0`
          (`/Engine/EditorBlueprintResources/StandardMacros.IsValid` _returnvalue
            (:`Is Valid`
              (if (not (`Pawn.IsLocallyControlled` _returnvalue))
                (bind _splayerstate (message `/Game/Genderfield/Core/Interfaces/BPI_SPlayerState.GetSPlayerState` (`Pawn.PlayerState` _returnvalue)))
                (bind _splayerstate_2 (message `/Game/Genderfield/Core/Interfaces/BPI_SPlayerState.GetSPlayerState` (`GameplayStatics.GetPlayerState` 0)))
                (switch `ERelation` (`SPlayerState.GetRelation` _splayerstate _splayerstate_2)
                  (:`Enemy`
                    (`PaperSpriteComponent.SetSprite` (`self.PaperSprite`) null)
                    (`WidgetComponent.SetWidget` (`self.Widget`) null))
                  (:`Ally`
                    (`PaperSpriteComponent.SetSpriteColor` (`self.PaperSprite`) (struct :`R` 0.25 :`G` 0.25 :`B` 1.0 :`A` 1.0)))
                  (:`Friend`
                    (`PaperSpriteComponent.SetSpriteColor` (`self.PaperSprite`) (struct :`R` 0.25 :`G` 1.0 :`B` 0.25 :`A` 1.0))))))))
        (:`then_1`
          (bind _aswbp_gadget (cast `/Game/Genderfield/Widgets/WBP_Gadget` (`WidgetComponent.GetWidget` (`self.Widget`))))
          (bind _output_get (set `self.WBP_Gadget` _aswbp_gadget))
          (set `/Game/Genderfield/Widgets/WBP_Gadget.GadgetTexture` (`self.GadgetTexture`) _output_get)
          (set `/Game/Genderfield/Widgets/WBP_Gadget.OwnerGadget` self _output_get))))))

(event `SInteractInterface.ShowInteractWidget`
  (bind _wbp_gadget (`self.WBP_Gadget`)
    (:`then`
      (`SBaseWidget.OnViewed` _wbp_gadget))
    (:`else`)))

(event `SInteractInterface.Interact`
  (params (Character :type "SCharacter Object Reference")))

(event `BeginCooldown`
  (bind _returnvalue (`KismetSystemLibrary.K2_SetTimerDelegate` (delegate `CooldownEnd`) (`self.CooldownTime`)))
  (set `self.CooldownTimer` _returnvalue))

(event `CooldownEnd`)

(fn `UserConstructionScript`)