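; Claymore weapon gadget that lets the owning character place a claymore in the world.
; MakeShoot traces a short distance from the owner's camera and, on a hit, spawns BP_GadgetWorld_Claymore at the impact point.
; Mostly upward-facing surfaces orient it along the character's forward vector, while steeper ones align its Z axis to the surface normal.
; Each placement uses up one charge and starts a ShootRate timer that calls StopShooting.
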(event `self.MakeShoot`
  (bind _bp_scharacter (message `/Game/Genderfield/Core/Interfaces/BPI_SCharacter.GetSCharacter` (`self.GetOwner`)))
  (bind _camera (`SCharacter.Camera` _bp_scharacter))
  (bind _returnvalue (`SceneComponent.K2_GetComponentLocation` _camera))
  (bind (_outhit _returnvalue_2) (`KismetSystemLibrary.LineTraceSingle` _returnvalue (+ _returnvalue (* (`SceneComponent.GetForwardVector` _camera) 250)) "TraceTypeQuery1" false (`|MakeArray` _bp_scharacter :!type "Actor Object Reference")))
  (if _returnvalue_2
    (bind (_bblockinghit _binitialoverlap _time _distance _location _impactpoint _normal _impactnormal) (`GameplayStatics.BreakHitResult` _outhit))
    (`|SpawnActorFromClass` "/Game/Genderfield/Gadget/BP_GadgetWorld_Claymore.BP_GadgetWorld_Claymore_C" (`KismetMathLibrary.MakeTransform` _impactpoint (`KismetMathLibrary.SelectRotator` (`KismetMathLibrary.MakeRotFromX` (`self.GetActorForwardVector` _bp_scharacter)) (`KismetMathLibrary.MakeRotFromZ` _impactnormal) (> (.z _impactnormal) 0.6))) "Undefined" "MultiplyWithRoot" self _bp_scharacter)
    (`/Engine/EditorBlueprintResources/StandardMacros.DecrementInt` (`self.LeftUsesAmount`)
      (:`  `
        (bind _returnvalue_3 (`KismetSystemLibrary.K2_SetTimer` null "StopShooting" (`self.ShootRate`)))
        (set `self.ShootTimer` _returnvalue_3)))))

(fn `UserConstructionScript`)