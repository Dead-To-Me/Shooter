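; Interactable door that swings between its initial rotation and an end rotation via a timeline.
; On authority, Interact toggles the Open flag, whose RepNotify plays or reverses the timeline, and multicasts a creak sound that only non-server instances play.
; On remote, Interact drives the same timeline through its own FlipFlop, moving the door locally without waiting for replication.
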(event `self.ReceiveBeginPlay`
  (`parent.ReceiveBeginPlay`)
  (set `self.StartRotation` (`self.K2_GetActorRotation`)))

(event `self.ReceiveTick`
  (params (DeltaSeconds :type "Float (single-precision)"))
  (`parent.ReceiveTick` DeltaSeconds))

(event `MulticastChangeDoorState`
  (if (not (`KismetSystemLibrary.IsServer`))
    (`GameplayStatics.PlaySoundAtLocation` "/Game/Genderfield/Sounds/A_zvuk-skripa-dveri.A_zvuk-skripa-dveri" (`self.K2_GetActorLocation`) (struct) 1.0 1.0 0.0 null null null null)))

(event `SInteractInterface.Interact`
  (params (Character :type "SCharacter Object Reference"))
  (`/Engine/EditorBlueprintResources/ActorMacros.Switch Has Authority`
    (:`Authority`
      (`self.MulticastChangeDoorState`)
      (bind _isa (`/Engine/EditorBlueprintResources/StandardMacros.FlipFlop`)
        (:`A`
          (set `self.bOpen` _isa))
        (:`B`
          (set `self.bOpen` _isa))))
    (:`Remote`
      (`/Engine/EditorBlueprintResources/StandardMacros.FlipFlop`
        (:`A`
          (bind (_direction _alpha) (`Timeline|DoorTimeline` :!label _label)
            (:`Update`
              (`self.K2_SetActorRotation` (`KismetMathLibrary.RLerp` (`self.StartRotation`) (`self.EndRotation`) _alpha)))))
        (:`B`
          (goto _label :!via `Reverse`))))))

(event `OnRepOpen`
  (if (`self.bOpen`)
    (goto _label)
    (else
      (goto _label :!via `Reverse`))))

(fn `OnRep_bOpen`
  (`self.OnRepOpen`))

(fn `UserConstructionScript`
  (`parent.UserConstructionScript`))