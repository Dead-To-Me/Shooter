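; Bipod attachment component for a firearm that detects when the weapon can rest on a surface below it.
; Shortly after BeginPlay, on authority only, it caches the owning weapon and its character, then starts a looping half-second timer.
; While the character is nearly stationary, a short downward Visibility trace, ignoring weapon and owner, sets the firearm's Bipod flag.
; Movement clears the flag.
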(event `self.ReceiveBeginPlay`
  (`KismetSystemLibrary.Delay` 0.2)
  (`/Engine/EditorBlueprintResources/ActorComponentMacros.Switch Has Authority`
    (:`Authority`
      (bind _assweapon_firearm (cast `SWeaponFirearm` (`self.GetOwner`)))
      (bind _output_get (set `self.WeaponFirearm` _assweapon_firearm))
      (bind _bp_scharacter (message `/Game/Genderfield/Core/Interfaces/BPI_SCharacter.GetSCharacter` (`Actor.GetOwner` _output_get)))
      (set `self.SCharacter` _bp_scharacter)
      (`self.SCharacter`
        (:`then`
          (set `self.IgnoreActors` (`|MakeArray` (`self.GetOwner`) (`Actor.GetOwner` (`self.GetOwner`))))
          (`KismetSystemLibrary.K2_SetTimerDelegate` (delegate `CheckIfOnBipod`) 0.5 true))
        (:`else`)))))

(event `CheckIfOnBipod`
  (bind _returnvalue (`self.K2_GetComponentLocation`))
  (if (not (> (`KismetMathLibrary.VSize` (`Actor.GetVelocity` (`self.SCharacter`))) 2.0))
    (bind (_outhit _returnvalue_2) (`KismetSystemLibrary.LineTraceSingle` _returnvalue (+ _returnvalue (* (`KismetMathLibrary.NegateVector` (`self.GetUpVector`)) 50)) "TraceTypeQuery1" false (`self.IgnoreActors`)))
    (set `SWeaponFirearm.bBipod` _returnvalue_2 (`self.WeaponFirearm`))
    (else
      (set `SWeaponFirearm.bBipod` false (`self.WeaponFirearm`)))))